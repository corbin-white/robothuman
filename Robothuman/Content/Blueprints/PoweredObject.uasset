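; PoweredObject is a base Blueprint for objects that can be powered on or off.
; PowerOn, PowerOff and TogglePoweredState set IsPowered and raise an UpdateState flag.
; Tick consumes that flag once and calls StateWhileOn or StateWhileOff, both empty here, so state responses run on the next tick after a change.
; GetIsPowered exposes the current state.
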(event `self.ReceiveTick`
  (params (DeltaSeconds :type "Float (single-precision)"))
  (if (`self.UpdateState`)
    (set `self.UpdateState` false)
    (if (`self.IsPowered`)
      (`self.State While On`)
      (else
        (`self.StateWhileOff`)))))

(event `Power On`
  (set `self.IsPowered` true)
  (set `self.UpdateState` true :!label _label))

(event `Power Off`
  (set `self.IsPowered` false)
  (goto _label))

(event `Toggle Powered State`
  (set `self.IsPowered` (not (`self.IsPowered`)))
  (goto _label))

(event `State While On`)

(event `StateWhileOff`)

(fn `GetIsPowered`
  (returns (NewParam :type Boolean))
  (return (`self.IsPowered`)))

(fn `UserConstructionScript`)