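; Lightning strike actor that waits out a countdown, then reveals itself for a set duration and destroys itself.
; An overlap sphere, sized in construction, gives a one-time random chance to retarget onto the first-person character's location, triggering the player's lightning hit immediately on overlap.
; Tick runs the countdown, teleports the strike to any new target, then activates it.
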(event `Update Coordinates`
  (params (`New Transform` :type "Transform Structure"))
  (if (not (`self.IsActivated`))
    (bind _output_get (set `self.CurrentCoordinates` `New Transform`))
    (`SceneComponent.K2_SetWorldTransform` (`self.DefaultSceneRoot`) _output_get false true)
    (set `self.IsWaitingForNewDestination` false)))

(event `self.ReceiveTick`
  (params (DeltaSeconds :type "Float (single-precision)"))
  (bind _timercountdown (`self.TimerCountdown`))
  (if (`self.IsWaitingForNewDestination`)
    (if (<= _timercountdown (`self.TimerLength`))
      (set `self.TimerCountdown` (+ DeltaSeconds _timercountdown))
      (elif (`self.HasRetargeted`)
        (`self.Update Coordinates` (`self.NewCoordinates`))
        (else
          (set `self.IsWaitingForNewDestination` false))))
    (else
      ;[1 1 1] "Activate"
      (set `self.IsActivated` true)
      (`self.SetActorHiddenInGame` false)
      (`KismetSystemLibrary.Delay` (`self.LightningDuration`))
      (`self.K2_DestroyActor`))))

(event `self.RetargetSphere.OnComponentBeginOverlap`
  (params (OverlappedComponent :type "PrimitiveComponent Object Reference") (OtherActor :type "Actor Object Reference") (OtherComp :type "PrimitiveComponent Object Reference") (OtherBodyIndex :type Integer) (bFromSweep :type Boolean) (SweepResult :type "HitResult Structure (by ref)"))
  ;[1 1 1] Retarget to Object (Player BP)
  (bind _asfirst_person_character (cast `/Game/FirstPersonBP/Blueprints/FirstPersonCharacter` OtherActor))
  (`/Engine/EditorBlueprintResources/StandardMacros.DoOnce` false
    (:`Completed`
      (if (<= (`KismetMathLibrary.RandomFloatInRange` -1.0 (- (`self.Chance`) 1.0)) 0.0)
        (set `self.HasRetargeted` true)
        (set `self.NewCoordinates` (`KismetMathLibrary.MakeTransform` (`self.K2_GetActorLocation` _asfirst_person_character) (.rotation (`self.CurrentCoordinates`)) (.scale (`self.CurrentCoordinates`))))
        ;[1 1 1] Damage To Player
        (bind _asfirst_person_character_2 (cast `/Game/FirstPersonBP/Blueprints/FirstPersonCharacter` (`GameplayStatics.GetPlayerCharacter` 0)))
        (`/Game/FirstPersonBP/Blueprints/FirstPersonCharacter.Hit By Lightening` _asfirst_person_character_2)))))

(fn `Get World Transform`
  (returns (NewParam :type "Transform Structure"))
  (return (`self.CurrentCoordinates`)))

(fn `UserConstructionScript`
  (set `self.CurrentCoordinates` (`SceneComponent.K2_GetComponentToWorld` (`self.DefaultSceneRoot`)))
  (`SphereComponent.SetSphereRadius` (`self.RetargetSphere`) (`self.RetargetRadius`) true))