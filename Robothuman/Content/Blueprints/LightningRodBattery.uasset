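; Lightning rod battery actor that stores a percentage charge, drained while the first-person character overlaps its DrainCapsule.
; Tick applies natural decay, feeds charge queued by ChargeBattery in gradually up to an overcharge limit, and discharges while flagged, lighting a PointLight.
; It also scales FullArrow and EmptyArrow on Z as a charge gauge, hiding the empty arrow at full charge.
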(event `self.ReceiveTick`
  (params (DeltaSeconds :type "Float (single-precision)"))
  (bind _emptyarrow (`self.EmptyArrow`))
  (bind _currentchargeaspercent (`self.CurrentChargeAsPercent`))
  (bind _currentchargeaspercent_2 (`self.CurrentChargeAsPercent`))
  (bind _returnvalue (* DeltaSeconds (`self.ChargeSpeed`)))
  (bind _returnvalue_2 (`KismetMathLibrary.MapRangeClamped` (/ (`self.CurrentChargeAsPercent`) 100.0) 0.0 1.0 0.0 1.0))
  (`|ExecutionSequence`
    (:`then_0`
      ;[1 0.9382 0.8811] Natural Decay
      (if (> _currentchargeaspercent_2 0.0)
        (set `self.CurrentChargeAsPercent` (- _currentchargeaspercent_2 (* DeltaSeconds (`self.NaturalDecayRate`))))))
    (:`then_1`
      ;[0.4076 1 0.6798] Is Adding Charge
      (if (> (`self.ChargeToAdd`) 0.0)
        (set `self.ChargeToAdd` (- (`self.ChargeToAdd`) _returnvalue))
        (if (< _currentchargeaspercent (+ (`self.AllowedOverchargeAmount`) 100.0))
          (set `self.CurrentChargeAsPercent` (+ _returnvalue _currentchargeaspercent)))))
    (:`then_2`
      ;[1 0.3101 0.3649] Is Discharging Battery (if charge exists)
      (if (`self.IsDischarging`)
        (if (<= (`self.CurrentChargeAsPercent`) 0.0)
          (set `self.IsDischarging` false)
          (else
            (set `self.CurrentChargeAsPercent` (- (`self.CurrentChargeAsPercent`) (* DeltaSeconds (`self.DischargeSpeed`))))
            (`SceneComponent.SetVisibility` (`self.PointLight`) true false)))
        (else
          (`SceneComponent.SetVisibility` (`self.PointLight`) false false))))
    (:`then_3`
      ;[0.4323 0.4323 0.4323] Update Battery Graphics
      (`SceneComponent.SetRelativeScale3D` (`self.FullArrow`) (`KismetMathLibrary.MakeVector` 1.0 1.0 _returnvalue_2))
      (`SceneComponent.SetRelativeScale3D` _emptyarrow (`KismetMathLibrary.MakeVector` 1.0 1.0 (- 1.0 _returnvalue_2)))
      (if (>= (`self.CurrentChargeAsPercent`) 100.0)
        (`SceneComponent.SetVisibility` _emptyarrow false true)
        (`SceneComponent.SetVisibility` _emptyarrow false true)
        (else
          (`SceneComponent.SetVisibility` _emptyarrow true true))))))

(event `ChargeBattery`
  (params (Percentage :type "Float (double-precision)"))
  (set `self.ChargeToAdd` Percentage))

(event `DischargeBattery`
  (set `self.IsDischarging` true))

(event `StopDischarge`
  (set `self.IsDischarging` false))

(event `self.DrainCapsule.OnComponentBeginOverlap`
  (params (OverlappedComponent :type "PrimitiveComponent Object Reference") (OtherActor :type "Actor Object Reference") (OtherComp :type "PrimitiveComponent Object Reference") (OtherBodyIndex :type Integer) (bFromSweep :type Boolean) (SweepResult :type "HitResult Structure (by ref)"))
  (if (== (`GameplayStatics.GetObjectClass` OtherActor) "/Game/FirstPersonBP/Blueprints/FirstPersonCharacter.FirstPersonCharacter_C")
    (`self.DischargeBattery`)))

(event `self.DrainCapsule.OnComponentEndOverlap`
  (params (OverlappedComponent :type "PrimitiveComponent Object Reference") (OtherActor :type "Actor Object Reference") (OtherComp :type "PrimitiveComponent Object Reference") (OtherBodyIndex :type Integer))
  (if (== (`GameplayStatics.GetObjectClass` OtherActor) "/Game/FirstPersonBP/Blueprints/FirstPersonCharacter.FirstPersonCharacter_C")
    (`self.StopDischarge`)))

(fn `UserConstructionScript`)