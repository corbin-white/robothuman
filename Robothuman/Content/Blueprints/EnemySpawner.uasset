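; EnemySpawner is an actor that spawns AI enemies at the location of its Box component, one per SpawnEnemies event call.
; Each call spawns only while the Spawned flag is unset and fewer than five actors of the Enemies class exist in the world.
; A NumEnemies counter tracks the spawner's own total and sets Spawned at five, permanently stopping further spawns.
; Nothing inside this Blueprint calls SpawnEnemies.
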(event `Spawn Enemies`
  (bind _outactors (`GameplayStatics.GetAllActorsOfClass` "/Game/Blueprints/Enemies.Enemies_C"))
  (if (`self.Spawned `)
    _
    (elif (< (`KismetArrayLibrary.Array_Length` _outactors) 5)
      (`AIBlueprintHelperLibrary.SpawnAIFromClass` "/Game/Blueprints/Enemies.Enemies_C" null (`SceneComponent.K2_GetComponentLocation` (`self.Box`)))
      (bind _output_get (set `self.NumEnemies` (+ (`self.NumEnemies`) 1)))
      (if (>= _output_get 5)
        (set `self.Spawned ` true)))))

(fn `UserConstructionScript`)