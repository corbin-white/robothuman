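; DemoLight is a Blueprint for a rect light that either fluctuates or holds a stable on or off state.
; While fluctuating, Tick flips IsPowered and raises UpdateState at random intervals under half a second, without touching visibility here.
; Otherwise, Tick sets RectLight visibility every frame from StableStateOnOff.
; TogglePoweredState ends fluctuation and copies DesiredState into that stable state.
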(event `self.ReceiveTick`
  (params (DeltaSeconds :type "Float (single-precision)"))
  (`parent.ReceiveTick` DeltaSeconds)
  (if (`self.FluctuatingState`)
    (set `self.FluctuatingCounter` (+ (`self.FluctuatingCounter`) DeltaSeconds))
    (if (>= (`self.FluctuatingCounter`) (`self.FluctuatingCurrentFrequency`))
      (set `self.IsPowered` (not (`self.IsPowered`)))
      (set `self.UpdateState` true)
      (set `self.FluctuatingCounter` 0.0)
      (set `self.FluctuatingCurrentFrequency` (`KismetMathLibrary.RandomFloatInRange` 0.0 0.5)))
    (elif (`self.StableStateOnOff`)
      (`self.State While On`)
      (else
        (`self.StateWhileOff`)))))

(event `self.State While On`
  (`SceneComponent.SetVisibility` (`self.RectLight`) true false))

(event `self.StateWhileOff`
  (`SceneComponent.SetVisibility` (`self.RectLight`) false false))

(event `self.Toggle Powered State`
  (set `self.FluctuatingState` false)
  (if (`self.DesiredState`)
    (set `self.StableStateOnOff` true)
    (else
      (set `self.StableStateOnOff` false))))

(fn `UserConstructionScript`
  (`parent.UserConstructionScript`))