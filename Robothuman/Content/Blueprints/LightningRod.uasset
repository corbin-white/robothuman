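; Lightning rod actor that pulls nearby lightning to itself to charge a target battery and lets the player collect electricity.
; Each Tick scans all LightningObjects, redirecting those whose LightningPos overlaps the grab sphere to LightningDestination and charging TargetBattery on every such frame.
; CollectRadius overlap enables player input and actor-level end overlap disables it, gating the E key call to CollectElectricity on the character.
; The construction script sizes the grab sphere from GrabLightningRadius.
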(event `self.ReceiveTick`
  (params (DeltaSeconds :type "Float (single-precision)"))
  (bind _outactors (`GameplayStatics.GetAllActorsOfClass` "/Game/Blueprints/LightningObject.LightningObject_C"))
  (for _array_element _outactors
    (if (`PrimitiveComponent.IsOverlappingComponent` (`self.GrabRadiusSphere`) (`/Game/Blueprints/LightningObject.LightningPos` _array_element))
      (`/Game/Blueprints/LightningObject.Update Coordinates` _array_element (`KismetMathLibrary.MakeTransform` (`SceneComponent.K2_GetComponentLocation` (`self.LightningDestination`))))
      (`/Game/Blueprints/LightningRodBattery.ChargeBattery` (`self.TargetBattery`) 25.0))))

(event `self.CollectRadius.OnComponentBeginOverlap`
  (params (OverlappedComponent :type "PrimitiveComponent Object Reference") (OtherActor :type "Actor Object Reference") (OtherComp :type "PrimitiveComponent Object Reference") (OtherBodyIndex :type Integer) (bFromSweep :type Boolean) (SweepResult :type "HitResult Structure (by ref)"))
  ;[1 1 1] Only Collect Lightning When in Range
  (cast `/Game/FirstPersonBP/Blueprints/FirstPersonCharacter` OtherActor)
  (`self.EnableInput` (`GameplayStatics.GetPlayerController` 0)))

(event `self.ReceiveActorEndOverlap`
  (params (OtherActor :type "Actor Object Reference"))
  ;[1 1 1] Only Collect Lightning When in Range
  (cast `/Game/FirstPersonBP/Blueprints/FirstPersonCharacter` OtherActor)
  (`self.DisableInput` (`GameplayStatics.GetPlayerController` 0)))

(event `Key|E`
  (params (Key :type "Key Structure"))
  ;[1 1 1] Collect Lightning
  (:`Pressed`
    (bind _asfirst_person_character (cast `/Game/FirstPersonBP/Blueprints/FirstPersonCharacter` (`GameplayStatics.GetPlayerCharacter` 0)))
    (`/Game/FirstPersonBP/Blueprints/FirstPersonCharacter.Collect Electricity` _asfirst_person_character)))

(fn `UserConstructionScript`
  (`SphereComponent.SetSphereRadius` (`self.GrabRadiusSphere`) (`self.GrabLightningRadius`) true))