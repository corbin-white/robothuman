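; EnemyDestroyer is an interactable actor that lets the player kill every enemy in the level at once.
; A Sphere trigger enables the actor's input while a FirstPersonCharacter overlaps it and disables it on exit.
; Pressing E then gathers all actors of the Enemies class and calls KillEnemy on them, behind a branch that is always true.
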(event `self.Sphere.OnComponentBeginOverlap`
  (params (OverlappedComponent :type "PrimitiveComponent Object Reference") (OtherActor :type "Actor Object Reference") (OtherComp :type "PrimitiveComponent Object Reference") (OtherBodyIndex :type Integer) (bFromSweep :type Boolean) (SweepResult :type "HitResult Structure (by ref)"))
  ;[1 1 1] When in Range
  (cast `/Game/FirstPersonBP/Blueprints/FirstPersonCharacter` OtherActor)
  (`self.EnableInput` (`GameplayStatics.GetPlayerController` 0)))

(event `self.Sphere.OnComponentEndOverlap`
  (params (OverlappedComponent :type "PrimitiveComponent Object Reference") (OtherActor :type "Actor Object Reference") (OtherComp :type "PrimitiveComponent Object Reference") (OtherBodyIndex :type Integer))
  ;[1 1 1] When in Range
  (cast `/Game/FirstPersonBP/Blueprints/FirstPersonCharacter` OtherActor)
  (`self.DisableInput` (`GameplayStatics.GetPlayerController` 0)))

(event `Key|E`
  (params (Key :type "Key Structure"))
  ;[1 1 1] Kill Enemies
  (:`Pressed`
    (if true
      (bind _outactors (`GameplayStatics.GetAllActorsOfClass` "/Game/Blueprints/Enemies.Enemies_C"))
      (`/Game/Blueprints/Enemies.Kill Enemy` _outactors))))

(fn `UserConstructionScript`)