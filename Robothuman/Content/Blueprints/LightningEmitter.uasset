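; Lightning emitter actor that periodically spawns LightningObject actors at random points inside a box volume around itself.
; Tick accumulates delta time and spawns once it exceeds the current interval, then resets the timer.
; Spawn points are random offsets within the RangeBox extents added to the root's world location, with no rotation.
; The construction script fixes the interval to the upper frequency value and sizes the box's X and Y from variables.
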(event `self.ReceiveTick`
  (params (DeltaSeconds :type "Float (single-precision)"))
  (bind _x (.x (`BoxComponent.BoxExtent` (`self.RangeBox`))))
  (bind _y (.y (`BoxComponent.BoxExtent` (`self.RangeBox`))))
  (bind _z (.z (`BoxComponent.BoxExtent` (`self.RangeBox`))))
  (`|ExecutionSequence`
    (:`then_0`
      (set `self.SpawnLightningCooldown` (+ DeltaSeconds (`self.SpawnLightningCooldown`))))
    (:`then_1`
      (if (> (`self.SpawnLightningCooldown`) (`self.SpawnLightningCurrentFrequency`))
        (`|SpawnActorFromClass` "/Game/Blueprints/LightningObject.LightningObject_C" (`KismetMathLibrary.MakeTransform` (`KismetMathLibrary.MakeVector` (+ (`KismetMathLibrary.RandomFloatInRange` (* _x -1.0) _x) (.x (.location (`SceneComponent.K2_GetComponentToWorld` (`self.DefaultSceneRoot`))))) (+ (`KismetMathLibrary.RandomFloatInRange` (* _y -1.0) _y) (.y (.location (`SceneComponent.K2_GetComponentToWorld` (`self.DefaultSceneRoot`))))) (+ (`KismetMathLibrary.RandomFloatInRange` (* _z -1.0) _z) (.z (.location (`SceneComponent.K2_GetComponentToWorld` (`self.DefaultSceneRoot`))))))) "Undefined" "OverrideRootScale" null null)
        (set `self.SpawnLightningCooldown` 0.0)))))

(fn `UserConstructionScript`
  (set `self.SpawnLightningCurrentFrequency` (`self.SpawnLightningUpperFrequency`))
  (`BoxComponent.SetBoxExtent` (`self.RangeBox`) (`KismetMathLibrary.MakeVector` (`self.RangeBoxX`) (`self.RangeBoxY`) (.z (`BoxComponent.BoxExtent` (`self.RangeBox`)))) false))